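; Player controller that prints debug text and holds request/response events that appear to exercise client-server messaging.
; On BeginPlay it prints the Count of every BP_ThirdPersonCharacter, and key 1 prints a fixed message and gathers all player controllers without using them.
; Req_Server calls Multicast on BP_ThirdPersonGameMode, then ResServer.
; The Res_Print, Res_Server and Req_PrintCount events are empty stubs.
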(event `self.ReceiveBeginPlay`
  (`self.PrintAllCharacterCount`))

(event `Req_Print`
  (`self.Req_Print`))

(event `Res_Print`)

(event `Key|One`
  (params (Key :type "Key Structure"))
  (:`Pressed`
    (`self.PrintData`)
    (bind _outactors (`GameplayStatics.GetAllActorsOfClass` "BP_PlayerController_C"))
    (set `self.Out Actors` _outactors)))

(event `Key|Two`
  (params (Key :type "Key Structure")))

(event `Req_PrintCount`)

(event `Req_Server`
  (bind _asbp_third_person_game_mode (cast `/Game/ThirdPerson/Blueprints/BP_ThirdPersonGameMode` (`GameplayStatics.GetGameMode`)))
  (`/Game/ThirdPerson/Blueprints/BP_ThirdPersonGameMode.Multicast` _asbp_third_person_game_mode)
  (`/Engine/EditorBlueprintResources/StandardMacros.IsValid` _asbp_third_person_game_mode
    (:`Is Valid`
      (`self.Res_Server`))))

(event `Key|Three`
  (params (Key :type "Key Structure")))

(event `Res_Server`)

(fn `PrintAllCharacterCount`
  (bind _outactors (`GameplayStatics.GetAllActorsOfClass` "/Game/ThirdPerson/Blueprints/BP_ThirdPersonCharacter.BP_ThirdPersonCharacter_C"))
  (for (_array_element _array_index) _outactors
    (`KismetSystemLibrary.PrintString` (`KismetStringLibrary.Concat_StrStr` "Player " (`KismetStringLibrary.Conv_IntToString` _array_index) " Count is " (`KismetStringLibrary.Conv_IntToString` (`/Game/ThirdPerson/Blueprints/BP_ThirdPersonCharacter.Count` _array_element))))))

(fn `PrintData`
  (`KismetSystemLibrary.PrintString` "This Function Called by PlayerController"))

(fn `UserConstructionScript`)